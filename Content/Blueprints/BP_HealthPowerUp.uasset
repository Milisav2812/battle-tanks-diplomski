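; Health pickup that restores a player tank's health when overlapped.
; On overlap it casts the other actor to BP_PlayerTank and does nothing if health is already full.
; Otherwise it adds Amount to the tank's Health CurrentHealth, capped at MaxHealth, then destroys itself.
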(event Collision|EventActorBeginOverlap
  (params (OtherActor :type Actor%20Object%20Reference))
  (bind _asbp_player_tank (Utilities|Casting|CastToBP_PlayerTank OtherActor))
  (if (not (== (Variables|/Script/BattleTanks.HealthComponent|GetCurrentHealth (Variables|/Game/Blueprints/Pawns/BP_PlayerTank.BP_PlayerTank_C|GetHealth _asbp_player_tank)) (Variables|/Script/BattleTanks.HealthComponent|GetMaxHealth (Variables|/Game/Blueprints/Pawns/BP_PlayerTank.BP_PlayerTank_C|GetHealth _asbp_player_tank))))
    (if (> (+ (Variables|/Script/BattleTanks.HealthComponent|GetCurrentHealth (Variables|/Game/Blueprints/Pawns/BP_PlayerTank.BP_PlayerTank_C|GetHealth _asbp_player_tank)) (Variables|Default|GetAmount)) (Variables|/Script/BattleTanks.HealthComponent|GetMaxHealth (Variables|/Game/Blueprints/Pawns/BP_PlayerTank.BP_PlayerTank_C|GetHealth _asbp_player_tank)))
      (Variables|/Script/BattleTanks.HealthComponent|SetCurrentHealth (Variables|/Game/Blueprints/Pawns/BP_PlayerTank.BP_PlayerTank_C|GetHealth _asbp_player_tank) (Variables|/Script/BattleTanks.HealthComponent|GetMaxHealth (Variables|/Game/Blueprints/Pawns/BP_PlayerTank.BP_PlayerTank_C|GetHealth _asbp_player_tank)))
      (else
        (Variables|/Script/BattleTanks.HealthComponent|SetCurrentHealth (Variables|/Game/Blueprints/Pawns/BP_PlayerTank.BP_PlayerTank_C|GetHealth _asbp_player_tank) (+ (Variables|/Script/BattleTanks.HealthComponent|GetCurrentHealth (Variables|/Game/Blueprints/Pawns/BP_PlayerTank.BP_PlayerTank_C|GetHealth _asbp_player_tank)) (Variables|Default|GetAmount)))))
    (Actor|DestroyActor)))

(fn ConstructionScript)