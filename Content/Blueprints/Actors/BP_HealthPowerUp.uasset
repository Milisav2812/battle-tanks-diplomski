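; BP_HealthPowerUp is a pickup actor that restores health to the player tank.
; On overlap with BP_PlayerTank, it does nothing if the tank's Health is already full, leaving the pickup in place.
; Otherwise it adds Amount to CurrentHealth, clamped to MaxHealth, then plays a 2D power-up sound and destroys itself.
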(event Collision|EventActorBeginOverlap
  (params (OtherActor :type Actor%20Object%20Reference))
  ;[1 1 1] Get Player Tank and check if Health is already full (CurrentHealth == MaxHealth)
  (bind _asbp_player_tank (Utilities|Casting|CastToBP_PlayerTank OtherActor))
  (if (not (== (Variables|/Script/BattleTanks.HealthComponent|GetCurrentHealth (Variables|/Game/Blueprints/Pawns/BP_PlayerTank.BP_PlayerTank_C|GetHealth _asbp_player_tank)) (Variables|/Script/BattleTanks.HealthComponent|GetMaxHealth (Variables|/Game/Blueprints/Pawns/BP_PlayerTank.BP_PlayerTank_C|GetHealth _asbp_player_tank))))
    ;[1 1 1] Increase CurrentHealth and check if its >= Max Health
    (if (> (+ (Variables|/Script/BattleTanks.HealthComponent|GetCurrentHealth (Variables|/Game/Blueprints/Pawns/BP_PlayerTank.BP_PlayerTank_C|GetHealth _asbp_player_tank)) (Variables|Default|GetAmount)) (Variables|/Script/BattleTanks.HealthComponent|GetMaxHealth (Variables|/Game/Blueprints/Pawns/BP_PlayerTank.BP_PlayerTank_C|GetHealth _asbp_player_tank)))
      ;[1 1 1] If it is, set CurrentHealth to MaxHealth
      (Variables|/Script/BattleTanks.HealthComponent|SetCurrentHealth (Variables|/Game/Blueprints/Pawns/BP_PlayerTank.BP_PlayerTank_C|GetHealth _asbp_player_tank) (Variables|/Script/BattleTanks.HealthComponent|GetMaxHealth (Variables|/Game/Blueprints/Pawns/BP_PlayerTank.BP_PlayerTank_C|GetHealth _asbp_player_tank)))
      (else
        (Variables|/Script/BattleTanks.HealthComponent|SetCurrentHealth (Variables|/Game/Blueprints/Pawns/BP_PlayerTank.BP_PlayerTank_C|GetHealth _asbp_player_tank) (+ (Variables|/Script/BattleTanks.HealthComponent|GetCurrentHealth (Variables|/Game/Blueprints/Pawns/BP_PlayerTank.BP_PlayerTank_C|GetHealth _asbp_player_tank)) (Variables|Default|GetAmount)))))
    (Audio|PlaySound2D "/Game/Assets/Sounds/PowerUp.PowerUp" 1.0 1.0 0.0 0 0)
    (Actor|DestroyActor)))

(fn ConstructionScript)