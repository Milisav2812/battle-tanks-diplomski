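; Game mode Blueprint for Battle Tanks that shows the start and end-of-match screens.
; The StartGame event creates the start game widget and adds it to the viewport.
; The GameOver event creates the end game widget, sets green win or red loss text from the GameWon flag, adds it to the viewport and enables the first player's mouse cursor.
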(event EventBeginPlay)

(event EventTick
  (params (DeltaSeconds :type Float%20%28single-precision%29)))

(event EventStartGame
  ;[1 1 1] Adding Start Widget to Viewport when StartGame is called
  (bind _returnvalue (UserInterface|CreateWidget "/Game/Blueprints/Widgets/WBP_StartGameWidget.WBP_StartGameWidget_C"))
  (UserInterface|Viewport|AddtoViewport _returnvalue 0))

(event EventGameOver
  (params (bGameWon :type Boolean))
  ;[1 1 1] Game Over Logic
  (bind _returnvalue (UserInterface|CreateWidget "/Game/Blueprints/Widgets/WBP_EndGameWidget.WBP_EndGameWidget_C"))
  (if bGameWon
    (Rendering|Components|TextRender|SetText (Variables|/Game/Blueprints/Widgets/WBP_EndGameWidget.WBP_EndGameWidget_C|GetDisplayText _returnvalue) "YOU WON!")
    (Appearance|SetColorandOpacity (Variables|/Game/Blueprints/Widgets/WBP_EndGameWidget.WBP_EndGameWidget_C|GetDisplayText _returnvalue) (Utilities|Struct|MakeSlateColor "(R=0.000000,G=0.479167,B=0.010888,A=1.000000)") :!class /Script/UMG.TextBlock)
    (else
      (Rendering|Components|TextRender|SetText (Variables|/Game/Blueprints/Widgets/WBP_EndGameWidget.WBP_EndGameWidget_C|GetDisplayText _returnvalue) "WASTED!")
      (Appearance|SetColorandOpacity (Variables|/Game/Blueprints/Widgets/WBP_EndGameWidget.WBP_EndGameWidget_C|GetDisplayText _returnvalue) (Utilities|Struct|MakeSlateColor "(R=0.432292,G=0.017937,B=0.000000,A=1.000000)") :!class /Script/UMG.TextBlock)))
  (UserInterface|Viewport|AddtoViewport _returnvalue 0)
  (Variables|/Script/Engine.PlayerController|SetbShowMouseCursor (Game|GetPlayerController 0) true))

(fn ConstructionScript)