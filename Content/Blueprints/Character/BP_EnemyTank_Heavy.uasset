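; Heavy enemy tank Blueprint that patrols one of four preset routes and shows its health on a widget bar.
; BeginPlay fills the bar, then picks a route from EnemyTankID, printing a warning if it is 0.
; Each route chains AIMoveTo calls through fixed locations and restarts only when every move succeeds.
; Tick refreshes the bar from the Health component while health is above zero.
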(event Custom|Patrol%20Event%201
  (bind _self self)
  ;[1 1 1] Patrol Event 1 - First Tank (Living Room)
  (AI|AIMoveTo _self (Variables|Patrol|GetLocation%201_1) 0 5.0 false
    (:OnSuccess
      (AI|AIMoveTo _self (Variables|Patrol|GetLocation%201_2) 0 5.0 false
        (:OnSuccess
          (AI|AIMoveTo _self (Variables|Patrol|GetLocation%201_3) 0 5.0 false
            (:OnSuccess
              (AI|AIMoveTo _self (Variables|Patrol|GetLocation%201_4) 0 5.0 false
                (:OnSuccess
                  (CallFunction|PatrolEvent1))))))))))

(event Custom|Patrol%20Event%204
  (bind _self self)
  ;[1 1 1] Patrol Event 4 - Third Tank (Labyrinth)
  (AI|AIMoveTo _self (Variables|Patrol|GetLocation%204_1) 0 5.0 false
    (:OnSuccess
      (AI|AIMoveTo _self (Variables|Patrol|GetLocation%204_2) 0 5.0 false
        (:OnSuccess
          (AI|AIMoveTo _self (Variables|Patrol|GetLocation%204_3) 0 5.0 false
            (:OnSuccess
              (AI|AIMoveTo _self (Variables|Patrol|GetLocation%204_2) 0 5.0 false
                (:OnSuccess
                  (CallFunction|PatrolEvent4))))))))))

(event Custom|Patrol%20Event%202
  (bind _self self)
  ;[1 1 1] Patrol Event 2 - First Tank (Labyrinth)
  (AI|AIMoveTo _self (Variables|Patrol|GetLocation%202_2) 0 5.0 false
    (:OnSuccess
      (AI|AIMoveTo _self (Variables|Patrol|GetLocation%202_1) 0 5.0 false
        (:OnSuccess
          (AI|AIMoveTo _self (Variables|Patrol|GetLocation%202_2) 0 5.0 false
            (:OnSuccess
              (AI|AIMoveTo _self (Variables|Patrol|GetLocation%202_4) 0 5.0 false
                (:OnSuccess
                  (AI|AIMoveTo _self (Variables|Patrol|GetLocation%202_3) 0 5.0 false
                    (:OnSuccess
                      (AI|AIMoveTo _self (Variables|Patrol|GetLocation%202_5) 0 5.0 false
                        (:OnSuccess
                          (AI|AIMoveTo _self (Variables|Patrol|GetLocation%202_3) 0 5.0 false
                            (:OnSuccess
                              (CallFunction|PatrolEvent2))))))))))))))))

(event Custom|Patrol%20Event%203
  (bind _self self)
  ;[1 1 1] Patrol Event 3 - Second Tank (Labyrinth)
  (AI|AIMoveTo _self (Variables|Patrol|GetLocation%203_1) 0 5.0 false
    (:OnSuccess
      (AI|AIMoveTo _self (Variables|Patrol|GetLocation%203_2) 0 5.0 false
        (:OnSuccess
          (CallFunction|PatrolEvent3))))))

(event EventBeginPlay
  ;[1 1 1] Initialize HealthBar to 100% & get HealthBar reference
  (bind _asenemy_health_bar (Utilities|Casting|CastToEnemyHealthBar (UserInterface|GetUserWidgetObject (Variables|Default|GetHealth%20Widget))))
  (bind _output_get (Variables|Default|SetHP%20Widget%20Reference _asenemy_health_bar))
  (Default|SetHealth _output_get 1.0 1.0)
  ;[1 1 1] Logic that selects the Patrol Event based on the Enemy Tank ID
  (switch int (Variables|Default|GetEnemyTankID)
    (:0
      (Development|PrintString "Tank ID not set!"))
    (:1
      (CallFunction|PatrolEvent1))
    (:2
      (CallFunction|PatrolEvent2))
    (:3
      (CallFunction|PatrolEvent3))
    (:4
      (CallFunction|PatrolEvent4))))

(event EventTick
  (params (DeltaSeconds :type Float%20%28single-precision%29))
  (bind _health (Variables|Default|GetHealth))
  (bind _currenthealth (Variables|/Script/BattleTanks.HealthComponent|GetCurrentHealth _health))
  ;[1 1 1] Update HealthBar if CurrentHealth > 0
  (if (not (<= _currenthealth 0.0))
    (Default|SetHealth (Variables|Default|GetHP%20Widget%20Reference) _currenthealth (Variables|/Script/BattleTanks.HealthComponent|GetMaxHealth _health))))

(fn ConstructionScript)