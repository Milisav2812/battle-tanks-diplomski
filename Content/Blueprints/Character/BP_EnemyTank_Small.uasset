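; Small enemy tank that patrols fixed routes in the living room and displays a health bar.
; BeginPlay sets up the health bar widget and picks a patrol event by tank ID, while Tick refreshes the bar from Health as long as it is above zero.
; Each patrol loops through chained AI MoveTo calls, with Patrol Macro setting waypoint flags that let the route re-enter at the current leg.
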(event Custom|Patrol%20Event%201
  ;[1 1 1] Patrol Event 1 - First Tank (Living Room)
  (if (Variables|Patrol|GetPatrol%20Location%201)
    (AI|AIMoveTo self (Variables|Patrol|GetLocation%201_1) 0 5.0 false
      (:OnSuccess
        (Utilities|PatrolMacro false true false false
          (:Out
            (AI|AIMoveTo self (Variables|Patrol|GetLocation%201_2) 0 5.0 false :!label _label
              (:OnSuccess
                (Utilities|PatrolMacro true false false false
                  (:Out
                    (CallFunction|PatrolEvent1)))))))))
    (elif (Variables|Patrol|GetPatrol%20Location%202)
      (goto _label))))

(event Custom|Patrol%20Event%202
  ;[1 1 1] Patrol Event 2 - Second Tank (Living Room)
  (if (Variables|Patrol|GetPatrol%20Location%201)
    (AI|AIMoveTo self (Variables|Patrol|GetLocation%201) 0 5.0 false
      (:OnSuccess
        (Utilities|PatrolMacro false true false false
          (:Out
            (AI|AIMoveTo self (Variables|Patrol|GetLocation%202) 0 5.0 false :!label _label
              (:OnSuccess
                (Utilities|PatrolMacro false false true false
                  (:Out
                    (AI|AIMoveTo self (Variables|Patrol|GetLocation%203) 0 5.0 false :!label _label_2
                      (:OnSuccess
                        (Utilities|PatrolMacro false false false true
                          (:Out
                            (AI|AIMoveTo self (Variables|Patrol|GetLocation%204) 0 5.0 false :!label _label_3
                              (:OnSuccess
                                (Utilities|PatrolMacro true false false false
                                  (:Out
                                    (CallFunction|PatrolEvent2)))))))))))))))))
    (elif (Variables|Patrol|GetPatrol%20Location%202)
      (goto _label)
      (elif (Variables|Patrol|GetPatrol%20Location%203)
        (goto _label_2)
        (elif (Variables|Patrol|GetPatrol%20Location%204)
          (goto _label_3))))))

(event EventBeginPlay
  ;[1 1 1] Initialize HealthBar to 100% & get HealthBar reference
  (bind _asenemy_health_bar (Utilities|Casting|CastToEnemyHealthBar (UserInterface|GetUserWidgetObject (Variables|Default|GetHealth%20Widget))))
  (bind _output_get (Variables|Default|SetHP%20Widget%20Reference _asenemy_health_bar))
  (Default|SetHealth _output_get 1.0 1.0)
  ;[1 1 1] Logic that selects the Patrol Event based on the Enemy Tank ID
  (switch int (Variables|Default|GetEnemyTankID)
    (:0
      (Development|PrintString "Tank ID not set!"))
    (:1
      (CallFunction|PatrolEvent1))
    (:2
      (CallFunction|PatrolEvent2))))

(event EventTick
  (params (DeltaSeconds :type Float%20%28single-precision%29))
  (bind _health (Variables|Default|GetHealth))
  ;[1 1 1] Update HealthBar if CurrentHealth > 0
  (if (not (<= (Variables|/Script/BattleTanks.HealthComponent|GetCurrentHealth _health) 0.0))
    (Default|SetHealth (Variables|Default|GetHP%20Widget%20Reference) (Variables|/Script/BattleTanks.HealthComponent|GetCurrentHealth _health) (Variables|/Script/BattleTanks.HealthComponent|GetMaxHealth _health))))

(fn ConstructionScript)