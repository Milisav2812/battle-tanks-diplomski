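; Level 1 medium enemy tank that patrols an endless loop through four locations, starting on BeginPlay.
; PatrolEvent uses four boolean flags to pick the current leg, then chains AIMoveTo calls from Location1 to Location4 before calling itself again.
; After each successful move, a Patrol macro sets all four flags to mark the next leg; failed moves have no handling.
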(event Custom|Patrol%20Event
  ;[1 1 1] Patrol
  (if (Variables|Patrol|GetPatrol%20Location%201)
    (AI|AIMoveTo self (Variables|Patrol|GetLocation%201) 0 5.0 false
      (:OnSuccess
        (Utilities|PatrolMacro false true false false
          (:Out
            (AI|AIMoveTo self (Variables|Patrol|GetLocation%202) 0 5.0 false :!label _label
              (:OnSuccess
                (Utilities|PatrolMacro false false true false
                  (:Out
                    (AI|AIMoveTo self (Variables|Patrol|GetLocation%203) 0 5.0 false :!label _label_2
                      (:OnSuccess
                        (Utilities|PatrolMacro false false false true
                          (:Out
                            (AI|AIMoveTo self (Variables|Patrol|GetLocation%204) 0 5.0 false :!label _label_3
                              (:OnSuccess
                                (Utilities|PatrolMacro true false false false
                                  (:Out
                                    (CallFunction|PatrolEvent)))))))))))))))))
    (elif (Variables|Patrol|GetPatrol%20Location%202)
      (goto _label)
      (elif (Variables|Patrol|GetPatrol%20Location%203)
        (goto _label_2)
        (elif (Variables|Patrol|GetPatrol%20Location%204)
          (goto _label_3))))))

(event EventBeginPlay
  (CallFunction|PatrolEvent))

(fn ConstructionScript)