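; BP_EnemyTank_Small_1_1 is a small Level 1 enemy tank that patrols back and forth between two locations.
; PatrolEvent starts on BeginPlay and uses two boolean flags to choose whether to AI MoveTo Location1 or Location2.
; Each successful move flips the flags through a Patrol macro, and reaching Location2 re-calls PatrolEvent to repeat the loop.
; Failed moves are not handled, so the patrol stops if one fails.
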(event Custom|Patrol%20Event
  (if (Variables|Patrol|GetPatrol%20Location%201)
    (AI|AIMoveTo self (Variables|Patrol|GetLocation%201) 0 5.0 false
      (:OnSuccess
        (Utilities|PatrolMacro false true
          (:Out
            (AI|AIMoveTo self (Variables|Patrol|GetLocation%202) 0 5.0 false :!label _label
              (:OnSuccess
                (Utilities|PatrolMacro true false
                  (:Out
                    (CallFunction|PatrolEvent)))))))))
    (elif (Variables|Patrol|GetPatrol%20Location%202)
      (goto _label))))

(event EventBeginPlay
  (CallFunction|PatrolEvent))

(fn ConstructionScript)